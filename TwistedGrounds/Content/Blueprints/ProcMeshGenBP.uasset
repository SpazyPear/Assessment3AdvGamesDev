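; Procedural mesh Blueprint that shows where the player is aiming on "ProcMesh"-tagged actors and triggers sculpting there.
; Each Tick predicts a projectile path from the pawn's "Muzzle" component along the camera's forward vector.
; A hit on a tagged actor moves the Decal to the impact point and stores the hit, otherwise HitSet clears.
; SculptEvent calls Sculpt, defined outside these graphs, only while HitSet is true; SculptFunc calls it unconditionally.
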(event Custom|Sculpt%20Event
  (if (Variables|Default|GetHitSet)
    (Class|ProcMeshSculpt|Sculpt)))

(event EventBeginPlay)

(event Collision|EventActorBeginOverlap
  (params (OtherActor :type Actor%20Object%20Reference)))

(event EventTick
  (params (DeltaSeconds :type Float%20%28single-precision%29))
  (bind _returnvalue (Game|Player|GetPlayerPawn 0))
  (Utilities|FlowControl|Sequence
    (:then_0
      (bind (_outhit _outpathpositions _outlasttracedestination _returnvalue_2) (Class|GameplayStatics|BlueprintPredictProjectilePathbyTraceChannel (Transformation|GetWorldLocation (Utilities|Array|Get(acopy) (Actor|GetComponentsbyTag _returnvalue "/Script/Engine.SceneComponent" "Muzzle"))) (* (Math|Vector|GetForwardVector (Actor|GetComponentbyClass _returnvalue "/Script/Engine.CameraComponent")) 6e+04) true 0.0 "ECC_WorldDynamic" false 0 "None" 1.0 15.0 2.0 22.0))
      (if _returnvalue_2
        (if (Actor|ActorHasTag (.HitActor (Collision|BreakHitResult _outhit)) "ProcMesh")
          (Transformation|SetWorldLocation (Variables|Default|GetDecal) (.ImpactPoint (Collision|BreakHitResult _outhit)) false true)
          (Variables|Default|SetHitResult _outhit)
          (Variables|Default|SetHitSet true)
          (else
            (Variables|Default|SetHitSet false :!label _label)))
        (else
          (goto _label))))))

(fn ConstructionScript)

(fn SculptFunc
  (Class|ProcMeshSculpt|Sculpt))